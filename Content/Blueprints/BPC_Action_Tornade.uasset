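; BPC_Action_Tornade is a board-game action that moves the executing player to a random cell on their board, like a tornado.
; Its Execute override calls the parent, rolls a random index within the board's cell count, prints it to screen, then places the player on that cell.
; BeginPlay and Tick are disabled stubs, so all logic lives in Execute.
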(fn `Execute`
  (params (Player :type "/Game/Blueprints/BP_Player Object Reference"))
  (locals (Destination :type Integer))
  (`parent.Execute` Player)
  (bind _output_get (set `local.Destination` (`KismetMathLibrary.RandomIntegerInRange` 0 (- (`/Game/Blueprints/BP_Board.GetCellCount` (`/Game/Blueprints/BP_Player.Board` Player)) 1))))
  (`KismetSystemLibrary.PrintString` (`KismetStringLibrary.Conv_IntToString` _output_get))
  (`/Game/Blueprints/BP_Player.PlaceOnCell` Player (`local.Destination`)))