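; BP_Board is a board Blueprint that holds an array of Cells and exposes simple functions to query it.
; GetCellByIndex returns the cell at an index, and GetCellCount returns the array length.
; TryMoveToCell only reports whether an index is valid and moves nothing.
; The event graph and construction script are empty, so the Cells array is not filled in these graphs.
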(fn `GetCellByIndex`
  (params (Index :type Integer))
  (returns (Cell :type "/Game/Blueprints/BP_Cell Object Reference"))
  (return (`|GetArrayItem` (`self.Cells`) Index)))

(fn `GetCellCount`
  (returns (Count :type Integer))
  (return (`KismetArrayLibrary.Array_Length` (`self.Cells`))))

(fn `TryMoveToCell`
  (params (Index :type Integer))
  (returns (CanMove :type Boolean))
  (return (`KismetArrayLibrary.Array_IsValidIndex` (`self.Cells`) Index)))

(fn `UserConstructionScript`)