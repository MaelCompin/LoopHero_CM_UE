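; Board-game player pawn that rolls the dice on Space and moves around a looping board of cells.
; If the board accepts the target, a recursive step event hops it cell by cell using a timeline lerp with a sine arc, then activates the landing cell.
; While a choice is pending, A and B place it on one of two portal cells.
; The active player's position is saved in the GameInstance and restored on BeginPlay.
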(event `Key|SpaceBar`
  (params (Key :type "Key Structure"))
  (:`Pressed`
    (`self.PrepareMove`)))

(event `self.ReceiveBeginPlay`
  (bind _gamedata (`self.GameData`))
  (bind _asbp_game_instance (cast `/Game/Blueprints/BP_GameInstance` (`GameplayStatics.GetGameInstance`)))
  (set `self.GameData` _asbp_game_instance)
  (bind _returnvalue (`GameplayStatics.GetActorOfClass` "/Game/Blueprints/BP_Board.BP_Board_C"))
  (set `self.Board` _returnvalue)
  (bind _returnvalue_2 (`GameplayStatics.GetActorOfClass` "/Game/Blueprints/BP_Dice.BP_Dice_C"))
  (set `self.Dice` _returnvalue_2)
  (`self.PlaceOnCell` (`|GetArrayItem` (`/Game/Blueprints/BP_GameInstance.PositionPlayer` _gamedata) (`/Game/Blueprints/BP_GameInstance.ActualPlayer` _gamedata)))
  (`self.EnableInput` (`GameplayStatics.GetPlayerController` 0)))

(event `StepToNextCell`
  (bind _returnvalue (mod (+ (`self.CurrentIndex`) 1) (`/Game/Blueprints/BP_Board.GetCellCount` (`self.Board`))))
  (if (> (`self.StepsRemaining`) 0)
    (bind _cell (`/Game/Blueprints/BP_Board.GetCellByIndex` (`self.Board`) _returnvalue))
    (set `self.EndLocation` (+ (`self.K2_GetActorLocation` _cell) (0.0 0.0 35.0)))
    (set `self.StartLocation` (`self.K2_GetActorLocation`))
    (bind (_direction _alpha) (`Timeline|HopTimeline` :!via `PlayFromStart`)
      (:`Update`
        (`self.K2_SetActorLocation` (+ (`KismetMathLibrary.VLerp` (`self.StartLocation`) (`self.EndLocation`) _alpha) (`KismetMathLibrary.MakeVector` 0.0 0.0 (* (`KismetMathLibrary.DegSin` (* _alpha 180.0)) (`self.JumpHeight`))))))
      (:`Finished`
        (set `self.CurrentIndex` _returnvalue)
        (`/Engine/EditorBlueprintResources/StandardMacros.DecrementInt` (`self.StepsRemaining`)
          (:`  `
            (`self.StepToNextCell`)))))
    (else
      (set `self.IsMoving` false)
      (`self.SavePosition`)
      (bind _cell_2 (`/Game/Blueprints/BP_Board.GetCellByIndex` (`self.Board`) (`self.CurrentIndex`)))
      (`/Game/Blueprints/BP_Cell.ActivateCell` _cell_2 self))))

(event `Key|One`
  (params (Key :type "Key Structure")))

(event `Key|A`
  (params (Key :type "Key Structure"))
  (:`Pressed`
    (if (`self.IsChoosing`)
      (set `self.IsChoosing` false)
      (`self.PlaceOnCell` (`self.PortalA`)))))

(event `Key|Two`
  (params (Key :type "Key Structure")))

(event `Key|B`
  (params (Key :type "Key Structure"))
  (:`Pressed`
    (if (`self.IsChoosing`)
      (set `self.IsChoosing` false)
      (`self.PlaceOnCell` (`self.PortalB`)))))

(fn `MoveToCell`
  (params (Index :type Integer))
  (bind _count (`/Game/Blueprints/BP_Board.GetCellCount` (`self.Board`)))
  (set `self.StepsRemaining` (mod (+ (- Index (`self.CurrentIndex`)) _count) _count))
  (set `self.IsMoving` true)
  (`self.StepToNextCell`))

(fn `PlaceOnCell`
  (params (Index :type Integer))
  (bind _output_get (set `self.CurrentIndex` Index))
  (bind _cell (`/Game/Blueprints/BP_Board.GetCellByIndex` (`self.Board`) _output_get))
  (`self.K2_SetActorLocation` (+ (`self.K2_GetActorLocation` _cell) (0.0 0.0 35.0)))
  (`self.SavePosition`))

(fn `PrepareMove`
  (if (not (or (`self.IsMoving`) (`self.IsChoosing`)))
    (bind _result (`/Game/Blueprints/BP_Dice.GetDiceResult` (`self.Dice`)))
    (`KismetSystemLibrary.PrintString` (`KismetStringLibrary.Conv_IntToString` _result))
    (bind _returnvalue (mod (+ (`self.CurrentIndex`) _result) (`/Game/Blueprints/BP_Board.GetCellCount` (`self.Board`))))
    (bind _canmove (`/Game/Blueprints/BP_Board.TryMoveToCell` (`self.Board`) _returnvalue))
    (if _canmove
      (`self.MoveToCell` _returnvalue)
      (else
        (`KismetSystemLibrary.PrintString` "Trop Loin !")))))

(fn `SavePosition`
  (bind _gamedata (`self.GameData`))
  (`KismetArrayLibrary.Array_Set` (`/Game/Blueprints/BP_GameInstance.PositionPlayer` _gamedata) (`/Game/Blueprints/BP_GameInstance.ActualPlayer` _gamedata) (`self.CurrentIndex`) true))

(fn `UserConstructionScript`)