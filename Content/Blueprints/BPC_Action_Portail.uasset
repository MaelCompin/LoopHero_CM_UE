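; Portal action component that offers the player a choice between two destinations.
; Its Execute override calls the parent, copies DestinationA and DestinationB onto the player's PortalA and PortalB, and flags the player as choosing.
; It prints a French on-screen prompt to press A or B; this file handles neither the input nor the travel.
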(fn `Execute`
  (params (Player :type "/Game/Blueprints/BP_Player Object Reference"))
  (`parent.Execute` Player)
  (set `/Game/Blueprints/BP_Player.PortalA` (`self.DestinationA`) Player)
  (set `/Game/Blueprints/BP_Player.PortalB` (`self.DestinationB`) Player)
  (set `/Game/Blueprints/BP_Player.IsChoosing` true Player)
  (`KismetSystemLibrary.PrintString` "Portail. \nAppuie sur A ou B."))